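; Actor that travels along a spline path, named as a conveyor belt element.
; On BeginPlay it grabs the first BP_SplinePath in the level and starts a timeline with play rate set to the inverse of STimeToComplete.
; Each update maps the timeline track to distance along the spline and sets the actor's transform, sampling location in world space and rotation in local space.
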(event `self.ReceiveBeginPlay`
  (bind _returnvalue (`GameplayStatics.GetActorOfClass` "/Game/Blueprints/BP_SplinePath.BP_SplinePath_C"))
  (set `self.splineRef` _returnvalue)
  (`self.Move Object`))

(event `Move Object`
  (bind _spline (`/Game/Blueprints/BP_SplinePath.Spline` (`self.splineRef`)))
  (`TimelineComponent.SetPlayRate` (`self.Move Object T`) (/ 1.0 (`self.sTimeToComplete`)))
  (bind (_direction _move_track) (`Timeline|Move Object T`)
    (:`Update`
      (bind _returnvalue (`KismetMathLibrary.Lerp` 0.0 (`SplineComponent.GetSplineLength` (`/Game/Blueprints/BP_SplinePath.Spline` (`self.splineRef`))) _move_track))
      (`self.K2_SetActorTransform` (`KismetMathLibrary.MakeTransform` (`SplineComponent.GetLocationAtDistanceAlongSpline` _spline _returnvalue "World") (`SplineComponent.GetRotationAtDistanceAlongSpline` _spline _returnvalue "Local"))))))

(fn `UserConstructionScript`)