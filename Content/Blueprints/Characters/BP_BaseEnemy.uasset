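; BP_BaseEnemy is a base enemy character that handles health, death and stuns.
; Direct hit, blast radius and acid damage events share SubtractHealth, though only blast damage first checks the dead flag.
; Lethal hit or blast damage calls EnemyKilled to ragdoll the mesh with a directional pelvis impulse, while acid death ragdolls without one.
; Stun zeroes walk speed temporarily, and debug prints report each event.
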(event `/Game/Blueprints/Interfaces/BPI_Damage.DirectHitDamage`
  (params (Damage :type "Float (double-precision)") (HitDirection :type "Vector Structure"))
  (`KismetSystemLibrary.PrintString` "Direct Hit Damage")
  (bind _healthfullydepleted_ (`self.SubtractHealth` Damage))
  (if _healthfullydepleted_
    (`self.EnemyKilled` HitDirection)
    (else
      (`KismetSystemLibrary.PrintString` (`KismetStringLibrary.Conv_DoubleToString` (`self.currentHealth`)) true true (struct :`R` 1.0 :`G` 0.036322 :`A` 1.0)))))

(event `/Game/Blueprints/Interfaces/BPI_Damage.BlastRadiusDamage`
  (params (Damage :type "Float (double-precision)") (RagdollDirection :type "Vector Structure"))
  (if (not (`self.enemyDead?`))
    (`KismetSystemLibrary.PrintString` "Blast Radius Damage")
    (bind _healthfullydepleted_ (`self.SubtractHealth` Damage))
    (if _healthfullydepleted_
      (`self.EnemyKilled` RagdollDirection)
      (else
        (`KismetSystemLibrary.PrintString` (`KismetStringLibrary.Conv_DoubleToString` (`self.currentHealth`)) true true (struct :`R` 1.0 :`G` 0.036322 :`A` 1.0))))))

(event `/Game/Blueprints/Interfaces/BPI_Damage.AcidDamage`
  (params (Damage :type "Float (double-precision)"))
  (`KismetSystemLibrary.PrintString` "Acid Damage")
  (bind _healthfullydepleted_ (`self.SubtractHealth` Damage))
  (if _healthfullydepleted_
    (`PrimitiveComponent.SetSimulatePhysics` (`self.Mesh`) true)
    (set `self.enemyDead?` true)
    (`KismetSystemLibrary.PrintString` "Enemy Dead" true true (struct :`R` 1.0 :`G` 0.036322 :`A` 1.0))
    (else
      (`KismetSystemLibrary.PrintString` (`KismetStringLibrary.Conv_DoubleToString` (`self.currentHealth`)) true true (struct :`R` 1.0 :`G` 0.036322 :`A` 1.0)))))

(event `/Game/Blueprints/Interfaces/BPI_Damage.Stun`
  (`KismetSystemLibrary.PrintString` "Enemy Stunned")
  (set `CharacterMovementComponent.MaxWalkSpeed` 0.0 (`self.CharacterMovement`))
  (`KismetSystemLibrary.Delay` 5.0)
  (set `CharacterMovementComponent.MaxWalkSpeed` (`self.normalSpeed`) (`self.CharacterMovement`)))

(fn `EnemyKilled`
  (params (RagdollDirection :type "Vector Structure"))
  (bind (_returnvalue_x _returnvalue_y) (`KismetMathLibrary.BreakVector` (* RagdollDirection 10000.0)))
  (`PrimitiveComponent.SetSimulatePhysics` (`self.Mesh`) true)
  (`PrimitiveComponent.AddImpulse` (`self.Mesh`) (`KismetMathLibrary.MakeVector` _returnvalue_x _returnvalue_y 5000.0) "pelvis" true)
  (set `self.enemyDead?` true)
  (`KismetSystemLibrary.PrintString` "Enemy Dead" true true (struct :`R` 1.0 :`G` 0.036322 :`A` 1.0)))

(fn `SubtractHealth`
  (params (DamageTaken :type "Float (double-precision)"))
  (returns (`HealthFullyDepleted?` :type Boolean))
  (bind _output_get (set `self.currentHealth` (- (`self.currentHealth`) DamageTaken)))
  (return (<= _output_get 0.0)))

(fn `UserConstructionScript`)