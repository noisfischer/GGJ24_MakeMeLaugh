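; BP_AcidPuddle is a short-lived area hazard that repeatedly damages nearby enemies with acid.
; On BeginPlay it plays a sound, spawns a Niagara goo effect, starts a looping damage timer, and destroys itself a few seconds later.
; Each tick of the timer runs a stationary multi-sphere trace on the Visibility channel and sends an AcidDamageMessage to hit actors tagged "enemy".
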(event `self.ReceiveBeginPlay`
  (`GameplayStatics.PlaySoundAtLocation` "/Game/Audio/SFX/Cue/Acid_Puddle_Cue.Acid_Puddle_Cue" (`self.K2_GetActorLocation`) (struct) 0.5 1.0 0.1 null null null null)
  (`NiagaraFunctionLibrary.SpawnSystemAtLocation` "/Game/PArticles/NS_AcidGoo.NS_AcidGoo" (`self.K2_GetActorLocation`))
  (`self.Acid`)
  (`KismetSystemLibrary.K2_SetTimerDelegate` (delegate `Acid`) 0.2 true)
  (`KismetSystemLibrary.Delay` 3.0)
  (`self.K2_DestroyActor`))

(event `Acid`
  (bind _returnvalue (`self.K2_GetActorLocation`))
  (bind (_outhits _returnvalue_2) (`KismetSystemLibrary.SphereTraceMulti` :`Start` _returnvalue :`End` _returnvalue :`Radius` 400.0 :`TraceChannel` "TraceTypeQuery1" :`DrawTime` 1.0))
  (if _returnvalue_2
    (for _array_element _outhits
      (bind (_bblockinghit _binitialoverlap _time _distance _location _impactpoint _normal _impactnormal _physmat _hitactor) (`GameplayStatics.BreakHitResult` _array_element))
      (if (`self.ActorHasTag` _hitactor "enemy")
        (message `/Game/Blueprints/Interfaces/BPI_Damage.AcidDamage` _hitactor 5.0)))))

(fn `UserConstructionScript`)