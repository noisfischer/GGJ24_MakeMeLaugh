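; Base projectile Blueprint that explodes on impact and damages enemies it hits directly.
; On component hit it spawns its particle emitter and explosion sound, and computes a direction from itself toward the hit actor.
; Actors tagged as enemy receive a direct-hit damage message carrying the damage and that direction, named for ragdoll use.
; The projectile destroys itself after any hit.
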(event `self.Projectile.OnComponentHit`
  (params (HitComponent :type "PrimitiveComponent Object Reference") (OtherActor :type "Actor Object Reference") (OtherComp :type "PrimitiveComponent Object Reference") (NormalImpulse :type "Vector Structure") (Hit :type "HitResult Structure (by ref)"))
  (set `self.HitActor` OtherActor)
  (set `self.RagdollDirection` (`KismetMathLibrary.GetForwardVector` (`KismetMathLibrary.FindLookAtRotation` (`self.K2_GetActorLocation`) (`self.K2_GetActorLocation` (`.HitActor` (`GameplayStatics.BreakHitResult` Hit))))))
  (`GameplayStatics.SpawnEmitterAtLocation` (`self.Emitter Template`) (`self.K2_GetActorLocation`) (struct) (`self.EmitterScale`))
  (`GameplayStatics.PlaySoundAtLocation` (`self.ExplosionSound`) (`self.K2_GetActorLocation`) (struct) 1.0 1.0 0.0 null null null null)
  (if (`self.ActorHasTag` (`self.HitActor`) "enemy")
    (message `/Game/Blueprints/Interfaces/BPI_Damage.DirectHitDamage` (`self.HitActor`) (`self.HitDamage`) (`self.RagdollDirection`))
    (`self.K2_DestroyActor`)
    (else
      (`self.K2_DestroyActor`))))

(fn `UserConstructionScript`)