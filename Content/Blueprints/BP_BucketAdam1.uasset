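; BP_BucketAdam1 is an actor that travels along the spline of a BP_SplinePath3 actor found in the level at BeginPlay.
; A timeline, with play rate set to the inverse of TimeToComplete, maps its track value to a distance between zero and the spline's length.
; Each update sets the actor's transform from that point, using world-space location but local-space spline rotation.
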(event `self.ReceiveBeginPlay`
  (bind _returnvalue (`GameplayStatics.GetActorOfClass` "/Game/Blueprints/BP_SplinePath3.BP_SplinePath3_C"))
  (set `self.Spline REF` _returnvalue)
  (`self.Move Object`))

(event `Move Object`
  (bind _spline (`/Game/Blueprints/BP_SplinePath2.Spline` (`self.Spline REF`)))
  (`TimelineComponent.SetPlayRate` (`self.Move Object T`) (/ 1.0 (`self.Time To Complete`)))
  (bind (_direction _newtrack_0) (`Timeline|Move Object T`)
    (:`Update`
      (bind _returnvalue (`KismetMathLibrary.Lerp` 0.0 (`SplineComponent.GetSplineLength` (`/Game/Blueprints/BP_SplinePath2.Spline` (`self.Spline REF`))) _newtrack_0))
      (`self.K2_SetActorTransform` (`KismetMathLibrary.MakeTransform` (`SplineComponent.GetLocationAtDistanceAlongSpline` _spline _returnvalue "World") (`SplineComponent.GetRotationAtDistanceAlongSpline` _spline _returnvalue "Local"))))))

(fn `UserConstructionScript`)