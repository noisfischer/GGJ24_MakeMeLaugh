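; BP_NPC is an NPC that the third-person character can interact with and that checks objects passed to it.
; Its sphere's overlap events set CanInteract on the character, on at begin and off at end, each gated by an overlap check against the character's mesh.
; RemovefromInventory compares the passed object with BP_Item1 and only prints whether it was correct; no inventory is changed here.
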(event `/Game/Blueprints/BPI_Inventory.Remove From Inventory`
  (params (Object :type "Actor Object Reference"))
  (if (== Object "/Game/Blueprints/Items/BP_Item1.BP_Item1")
    (`KismetSystemLibrary.PrintString` "That was the correct object")
    (else
      (`KismetSystemLibrary.PrintString` "That was not the correct object"))))

(event `self.Sphere.OnComponentBeginOverlap`
  (params (OverlappedComponent :type "PrimitiveComponent Object Reference") (OtherActor :type "Actor Object Reference") (OtherComp :type "PrimitiveComponent Object Reference") (OtherBodyIndex :type Integer) (bFromSweep :type Boolean) (SweepResult :type "HitResult Structure (by ref)"))
  (bind _asbp_third_person_character (cast `/Game/ThirdPerson/Blueprints/BP_ThirdPersonCharacter` OtherActor :!pure true))
  (if (`PrimitiveComponent.IsOverlappingComponent` OverlappedComponent (`Character.Mesh` _asbp_third_person_character))
    (set `/Game/ThirdPerson/Blueprints/BP_ThirdPersonCharacter.canInteract` true _asbp_third_person_character)))

(event `self.Sphere.OnComponentEndOverlap`
  (params (OverlappedComponent :type "PrimitiveComponent Object Reference") (OtherActor :type "Actor Object Reference") (OtherComp :type "PrimitiveComponent Object Reference") (OtherBodyIndex :type Integer))
  (bind _asbp_third_person_character (cast `/Game/ThirdPerson/Blueprints/BP_ThirdPersonCharacter` OtherActor :!pure true))
  (if (`PrimitiveComponent.IsOverlappingComponent` OverlappedComponent (`Character.Mesh` _asbp_third_person_character))
    (set `/Game/ThirdPerson/Blueprints/BP_ThirdPersonCharacter.canInteract` false _asbp_third_person_character)))

(fn `UserConstructionScript`)