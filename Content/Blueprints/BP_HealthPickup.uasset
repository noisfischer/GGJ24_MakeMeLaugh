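; BP_HealthPickup is a short-lived pickup that heals the player character on overlap.
; On overlap with player 0's character it calls HealPlayerMessage on that character, spawns a green hit Niagara effect, plays a pop sound and destroys itself.
; If left uncollected, a delay started at BeginPlay destroys it after a few seconds with the same effect but no sound or heal.
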(event `self.ReceiveBeginPlay`
  (`KismetSystemLibrary.Delay` 5.0)
  (`NiagaraFunctionLibrary.SpawnSystemAtLocation` "/Game/PArticles/NS_HitGreen.NS_HitGreen" (`self.K2_GetActorLocation`))
  (`self.K2_DestroyActor`))

(event `self.ReceiveActorBeginOverlap`
  (params (OtherActor :type "Actor Object Reference"))
  (if (== OtherActor (`GameplayStatics.GetPlayerCharacter` 0))
    (message `/Game/Blueprints/Interfaces/BPI_Damage.HealPlayer` (`GameplayStatics.GetPlayerCharacter` 0))
    (`NiagaraFunctionLibrary.SpawnSystemAtLocation` "/Game/PArticles/NS_HitGreen.NS_HitGreen" (`self.K2_GetActorLocation`))
    (`GameplayStatics.PlaySound2D` "/Game/Audio/SFX/Cue/Pop_Cue.Pop_Cue" 1.0 1.0 0.0 null null)
    (`self.K2_DestroyActor`)))

(fn `UserConstructionScript`)