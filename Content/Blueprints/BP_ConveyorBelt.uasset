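; BP_ConveyorBelt is a conveyor belt actor that snaps back to a start location whenever it passes an end location.
; BeginPlay places it at StartLocation, and Tick repeats that unswept move once its X or Y exceeds the matching EndLocation coordinate.
; The graphs contain only this wrap-around reset, with no logic that advances the actor along the belt.
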(event `self.ReceiveTick`
  (params (DeltaSeconds :type "Float (single-precision)"))
  (if (or (> (.x (`self.K2_GetActorLocation`)) (.x (`self.endLocation`))) (> (.y (`self.K2_GetActorLocation`)) (.y (`self.endLocation`))))
    (`self.K2_SetActorLocation` (`self.startLocation`) :!label _label)))

(event `self.ReceiveBeginPlay`
  (goto _label))

(fn `UserConstructionScript`)