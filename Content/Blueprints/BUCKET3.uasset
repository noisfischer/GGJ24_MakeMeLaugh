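; BUCKET3 is an actor Blueprint meant to move itself along the spline of a BP_SplinePath3 actor.
; On BeginPlay it finds and stores that actor, then calls a MoveObject event that is empty.
; The disconnected timeline logic would travel the spline's length over TimeToComplete, taking world location at the lerped distance but local rotation always at distance zero.
; As wired, the actor does not move.
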(event `self.ReceiveBeginPlay`
  (bind _returnvalue (`GameplayStatics.GetActorOfClass` "/Game/Blueprints/BP_SplinePath3.BP_SplinePath3_C"))
  (set `self.Spline REF` _returnvalue)
  (`self.MoveObject`))

(event `MoveObject`)

(fn `UserConstructionScript`)