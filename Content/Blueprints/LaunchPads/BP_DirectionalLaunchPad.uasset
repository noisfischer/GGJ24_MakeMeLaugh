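; Launch pad actor that flings the first player's character in a configurable direction when it overlaps the pad.
; The construction script orients the LaunchDirection component in world space from the upward pitch and forward yaw variables, so the actor's own rotation does not steer the launch.
; On overlap, LaunchCharacter applies that component's forward vector scaled by LaunchForce, adding to existing velocity rather than overriding it.
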(event `self.ReceiveActorBeginOverlap`
  (params (OtherActor :type "Actor Object Reference"))
  (bind _returnvalue (`GameplayStatics.GetPlayerCharacter` 0))
  (if (== OtherActor _returnvalue)
    (`Character.LaunchCharacter` _returnvalue (* (`SceneComponent.GetForwardVector` (`self.LaunchDirection`)) (`self.LaunchForce`)) false false)))

(fn `UserConstructionScript`
  (`SceneComponent.K2_SetWorldRotation` (`self.LaunchDirection`) (`KismetMathLibrary.MakeRotator` 0.0 (`self.LaunchUpwardDirection`) (`self.LaunchForwardDirection`)) false false))