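; BP_Item1 is an item actor that signals the player character when it can be picked up.
; When a third-person character's mesh begins overlapping its Sphere, it passes itself to player 0's character via AddToInventoryMessage, then sets the overlapping character's CanPickup flag.
; Ending that mesh overlap clears the flag; inventory handling and the pickup itself are left to the receiving character.
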(event `self.Sphere.OnComponentBeginOverlap`
  (params (OverlappedComponent :type "PrimitiveComponent Object Reference") (OtherActor :type "Actor Object Reference") (OtherComp :type "PrimitiveComponent Object Reference") (OtherBodyIndex :type Integer) (bFromSweep :type Boolean) (SweepResult :type "HitResult Structure (by ref)"))
  (bind _asbp_third_person_character (cast `/Game/Blueprints/Characters/BP_ThirdPersonCharacter` OtherActor :!pure true))
  (if (== OtherComp (`Character.Mesh` _asbp_third_person_character))
    (message `/Game/Blueprints/Interfaces/BPI_Inventory.Add To Inventory` (`GameplayStatics.GetPlayerCharacter` 0) (`ActorComponent.GetOwner` OverlappedComponent))
    (set `/Game/Blueprints/Characters/BP_ThirdPersonCharacter.canPickup` true _asbp_third_person_character)))

(event `self.Sphere.OnComponentEndOverlap`
  (params (OverlappedComponent :type "PrimitiveComponent Object Reference") (OtherActor :type "Actor Object Reference") (OtherComp :type "PrimitiveComponent Object Reference") (OtherBodyIndex :type Integer))
  (bind _asbp_third_person_character (cast `/Game/Blueprints/Characters/BP_ThirdPersonCharacter` OtherActor :!pure true))
  (if (== OtherComp (`Character.Mesh` _asbp_third_person_character))
    (set `/Game/Blueprints/Characters/BP_ThirdPersonCharacter.canPickup` false _asbp_third_person_character)))

(fn `UserConstructionScript`)