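; BP_HomingProjectile is a projectile that homes in on a tagged enemy detected by its HomingTracking overlap component.
; Each overlap stores the other actor as EnemyTarget and prints a debug message, before any tag check.
; If that actor has the "enemy" tag, its root becomes the ProjectileMovement homing target and HomingTracking is destroyed, locking the target.
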(event `self.ReceiveBeginPlay`
  (`parent.ReceiveBeginPlay`))

(event `self.HomingTracking.OnComponentBeginOverlap`
  (params (OverlappedComponent :type "PrimitiveComponent Object Reference") (OtherActor :type "Actor Object Reference") (OtherComp :type "PrimitiveComponent Object Reference") (OtherBodyIndex :type Integer) (bFromSweep :type Boolean) (SweepResult :type "HitResult Structure (by ref)"))
  ;[1 1 1] Select Target
  (set `self.EnemyTarget` OtherActor)
  (`KismetSystemLibrary.PrintString` "Target Selected" true true (struct :`R` 1.0 :`B` 0.037106 :`A` 1.0))
  (if (`self.ActorHasTag` OtherActor "enemy")
    (set `ProjectileMovementComponent.HomingTargetComponent` (`Actor.RootComponent` (`self.EnemyTarget`)) (`self.ProjectileMovement`))
    (`ActorComponent.K2_DestroyComponent` (`self.HomingTracking`))))

(fn `UserConstructionScript`
  (`parent.UserConstructionScript`))